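; Player-controlled tank Pawn Blueprint that binds input to its aiming and movement components.
; BeginPlay passes the turret and barrel to TankAim and both tracks to TankNavMovement.
; Aim axes rotate the spring arm and azimuth gimbal at a frame-rate-independent speed to steer the camera.
; Fire calls TankAim and plays a 2D explosion sound, while move and turn axes forward intent to TankNavMovement.
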(event EventBeginPlay
  ;[1 1 1] Set the TankBarrel and TankTurret
  (Class|TankAimComponent|SetTankTurretBarrel (Variables|Default|GetTankAim) (Variables|Default|GetTank%20Turret) (Variables|Default|GetTank%20Barrel))
  (Class|TankNavMovementComponent|SetTracks (Variables|Default|GetTankNavMovement) (Variables|Default|GetLeft%20Tracks) (Variables|Default|GetRight%20Tracks)))

(event Collision|EventActorBeginOverlap
  (params (OtherActor :type Actor%20Object%20Reference)))

(event EventTick
  (params (DeltaSeconds :type Float%20%28single-precision%29)))

(event Input|ActionEvents|InputActionFire
  (params (Key :type Key%20Structure))
  ;[1 1 1] Firing
  (:Pressed
    (Class|TankAimComponent|Fire (Variables|Default|GetTankAim))
    (Audio|PlaySound2D "/Game/StarterContent/Audio/Explosion01.Explosion01" 1.0 1.0 0.0 0 0)))

(event Input|AxisEvents|InputAxisAimAzimuth
  (params (AxisValue :type Float%20%28single-precision%29))
  ;[1 1 1] Camera Rotation Reflect
  (Transformation|AddLocalRotation (Variables|Default|GetAzimuth%20Gimbal) (Math|Rotator|MakeRotator 0.0 0.0 (* (Utilities|Time|GetWorldDeltaSeconds) AxisValue 4e+01)) false false))

(event Input|AxisEvents|InputAxisAimElevation
  (params (AxisValue :type Float%20%28single-precision%29))
  ;[1 1 1] Camera Rotation Reflect
  (Transformation|AddLocalRotation (Variables|Default|GetSpringArm) (Math|Rotator|MakeRotator 0.0 (* AxisValue (Utilities|Time|GetWorldDeltaSeconds) 4e+01) 0.0) false false))

(event Input|AxisEvents|InputAxisTurnRight
  (params (AxisValue :type Float%20%28single-precision%29))
  ;[1 1 1] Moving Reflect
  (Class|TankNavMovementComponent|IntendTurnRight (Variables|Default|GetTankNavMovement) AxisValue))

(event Input|AxisEvents|InputAxisMoveForward
  (params (AxisValue :type Float%20%28single-precision%29))
  ;[1 1 1] Moving Reflect
  (Class|TankNavMovementComponent|IntendMoveForward (Variables|Default|GetTankNavMovement) AxisValue))

(fn ConstructionScript)