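; Tank pawn Blueprint that registers its barrel and turns player aim input into camera rotation.
; On BeginPlay it passes its Barrel to SetTankBarrel.
; AimAzimuth yaws the AzimuthGimbal while AimElevation pitches the SpringArm, keeping the two axes on separate components, both scaled by delta time for frame-rate-independent speed.
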(event EventBeginPlay)

(event Collision|EventActorBeginOverlap
  (params (OtherActor :type Actor%20Object%20Reference)))

(event EventTick
  (params (DeltaSeconds :type Float%20%28single-precision%29)))

(event EventBeginPlay
  ;[1 1 1] Set Tank Barrel
  (Class|Tank|SetTankBarrel (Variables|Default|GetBarrel)))

(event Input|AxisEvents|InputAxisAimAzimuth
  (params (AxisValue :type Float%20%28single-precision%29))
  ;[1 1 1] Camera Rotation Reflect
  (Transformation|AddLocalRotation (Variables|Default|GetAzimuth%20Gimbal) (Math|Rotator|MakeRotator 0.0 0.0 (* (Utilities|Time|GetWorldDeltaSeconds) AxisValue 4e+01)) false false))

(event Input|AxisEvents|InputAxisAimElevation
  (params (AxisValue :type Float%20%28single-precision%29))
  ;[1 1 1] Camera Rotation Reflect
  (Transformation|AddLocalRotation (Variables|Default|GetSpringArm) (Math|Rotator|MakeRotator 0.0 (* AxisValue (Utilities|Time|GetWorldDeltaSeconds) 4e+01) 0.0) false false))

(fn ConstructionScript)